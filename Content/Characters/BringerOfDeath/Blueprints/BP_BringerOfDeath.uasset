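; Blueprint for the Bringer of Death enemy character, whose death wins the game.
; On BeginPlay it caches the WBP_Enemy widget from HPWidget and binds to its health, max health and death events.
; Health changes update the bar as a safe current-to-max ratio.
; Death hides the bar, deactivates the player's BP_Knight, shows the WBP_Win screen and enables the mouse cursor.
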(event `OnMaxHealthChanged_Event`
  (params (newValue :type "Float (single-precision)"))
  (bind _output_get (set `self.MaxHealth` newValue))
  (`/Game/UI/WBP_Enemy.SetHealth` (`self.As WBP Enemy`) (`KismetMathLibrary.SafeDivide` (`self.CurrentHealth`) _output_get)))

(event `self.ReceiveBeginPlay`
  (`|ExecutionSequence`
    (:`then_0`
      (bind _aswbp_enemy (cast `/Game/UI/WBP_Enemy` (`WidgetComponent.GetWidget` (`self.HPWidget`))))
      (set `self.As WBP Enemy` _aswbp_enemy))
    (:`then_1`
      (add `EnemyCharacter.OnMaxHealthChanged` (delegate `OnMaxHealthChanged_Event`)))
    (:`then_2`
      (add `EnemyCharacter.OnHealthChanged` (delegate `OnHealthChanged_Event`)))
    (:`then_3`
      (add `self.OnDeath` (delegate `OnDeath_Event`)))))

(event `OnHealthChanged_Event`
  (params (newValue :type "Float (single-precision)"))
  (bind _output_get (set `self.CurrentHealth` newValue))
  (`/Game/UI/WBP_Enemy.SetHealth` (`self.As WBP Enemy`) (`KismetMathLibrary.SafeDivide` _output_get (`self.MaxHealth`))))

(event `OnDeath_Event`
  (`Widget.SetVisibility` (`self.As WBP Enemy`) "Hidden")
  (bind _asbp_knight (cast `/Game/Characters/Knight/Blueprints/BP_Knight` (`GameplayStatics.GetPlayerCharacter` 0)))
  (`KnightCharacter.Deactivate` _asbp_knight)
  (bind _returnvalue (`|CreateWidget` "/Game/UI/WBP_Win.WBP_Win_C"))
  (`UserWidget.AddToViewport` _returnvalue 0)
  (set `PlayerController.bShowMouseCursor` true (`GameplayStatics.GetPlayerController` 0)))

(fn `UserConstructionScript`)