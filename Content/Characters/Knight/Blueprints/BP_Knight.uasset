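; BP_Knight is the Knight character Blueprint, which shows a player health widget on screen.
; On BeginPlay it creates WBP_Player, stores it, adds it to the viewport and sets its health to the CurrentHP-to-MaxHP ratio.
; AnyDamage pushes that ratio to the widget again, without changing CurrentHP in this graph.
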(event `self.ReceiveBeginPlay`
  (bind _returnvalue (`|CreateWidget` "/Game/UI/WBP_Player.WBP_Player_C"))
  (bind _output_get (set `self.PlayerWidget` _returnvalue))
  (`UserWidget.AddToViewport` _output_get 0)
  (`/Game/UI/WBP_Player.SetHealth` (`self.PlayerWidget`) (/ (`self.CurrentHP`) (`self.MaxHP`))))

(event `self.ReceiveAnyDamage`
  (params (Damage :type "Float (single-precision)") (DamageType :type "DamageType Object Reference") (InstigatedBy :type "Controller Object Reference") (DamageCauser :type "Actor Object Reference"))
  (`/Game/UI/WBP_Player.SetHealth` (`self.PlayerWidget`) (/ (`self.CurrentHP`) (`self.MaxHP`))))

(fn `UserConstructionScript`)