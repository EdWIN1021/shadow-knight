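; BP_NightBorne is the NightBorne enemy character Blueprint, which keeps its HP widget in sync with its health.
; On BeginPlay it caches the HPWidget's WBP_Enemy instance and binds to the max health and current health change delegates.
; Each callback stores the new value and sends the current-to-max ratio to the widget, using a safe divide to guard against zero max health.
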(event `self.ReceiveBeginPlay`
  (`|ExecutionSequence`
    (:`then_0`
      (bind _aswbp_enemy (cast `/Game/UI/WBP_Enemy` (`WidgetComponent.GetWidget` (`self.HPWidget`))))
      (set `self.As WBP Enemy` _aswbp_enemy))
    (:`then_1`
      (add `self.OnMaxHealthChanged` (delegate `OnMaxHealthChanged_Event`)))
    (:`then_2`
      (add `self.OnHealthChanged` (delegate `OnHealthChanged_Event`)))))

(event `OnMaxHealthChanged_Event` :!signature `self.OnMaxHealthChanged`
  (params (newValue :type "Float (single-precision)"))
  (bind _output_get (set `self.MaxHealth` newValue))
  (`/Game/UI/WBP_Enemy.SetHealth` (`self.As WBP Enemy`) (`KismetMathLibrary.SafeDivide` (`self.CurrentHealth`) _output_get)))

(event `OnHealthChanged_Event` :!signature `self.OnHealthChanged`
  (params (newValue :type "Float (single-precision)"))
  (bind _output_get (set `self.CurrentHealth` newValue))
  (`/Game/UI/WBP_Enemy.SetHealth` (`self.As WBP Enemy`) (`KismetMathLibrary.SafeDivide` _output_get (`self.MaxHealth`))))

(fn `UserConstructionScript`)